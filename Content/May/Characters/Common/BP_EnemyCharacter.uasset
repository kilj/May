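; BP_EnemyCharacter is the enemy character Blueprint, adding an overhead-style status bar and motion-warped facing to its parent class.
; On BeginPlay it passes its May ability system component and attribute set to the status bar widget.
; Tick turns that widget toward the player camera in pitch only, with yaw fixed.
; SetFacingTarget calls the parent, then updates the FacingTarget motion warp location.
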(event EventBeginPlay
  (bind _aswbp_status_bar (Utilities|Casting|CastToWBP_StatusBar (UserInterface|GetUserWidgetObject (Variables|Default|GetStatusBarWidgetComponent))))
  (bind _data (CallFunction|CreateStatusBarWidgetData))
  (Class|StatusBarWidget|InitWidget _aswbp_status_bar _data))

(event EventTick
  (params (DeltaSeconds :type Float%20%28single-precision%29))
  (bind _statusbarwidgetcomponent (Variables|Default|GetStatusBarWidgetComponent)
    (:then
      (Utilities|IsValid (Game|GetPlayerCameraManager 0)
        (:Is%20Valid
          (Transformation|SetWorldRotation _statusbarwidgetcomponent (Math|Rotator|MakeRotator 0.0 (.pitch (Math|Rotator|FindLookatRotation (Transformation|GetWorldLocation (Variables|Default|GetStatusBarWidgetComponent)) (Transformation|GetWorldLocation (Variables|/Script/Engine.PlayerCameraManager|GetTransformComponent (Game|GetPlayerCameraManager 0))))) 1.8e+02) false false))))
    (:else)))

(event Collision|EventActorBeginOverlap
  (params (OtherActor :type Actor%20Object%20Reference)))

(event EventSetFacingTarget
  (params (Target :type Vector%20%28by%20ref%29 :default "0, 0, 0"))
  (|CallParentFunction Target)
  (Class|MotionWarpingComponent|AddorUpdateWarpTargetfromLocation (Variables|Default|GetMotionWarping) "FacingTarget" Target))

(fn ConstructionScript)

(fn CreateStatusBarWidgetData
  (bind _asmay_ability_system_component (Utilities|Casting|CastToMayAbilitySystemComponent (Class|MayCharacterBase|GetAbilitySystemComponent))
    (:then
      (LocalVariables|SetMayASC _asmay_ability_system_component)
      (bind _asmay_attribute_set (Utilities|Casting|CastToMayAttributeSet (Class|MayCharacterBase|GetAttributeSet))
        (:then
          (LocalVariables|SetMayAS _asmay_attribute_set)
          (return (Utilities|Struct|MakeStatusBarWidgetData (LocalVariables|GetMayASC) (LocalVariables|GetMayAS))))
        (:CastFailed
          (Development|PrintString "Cannot cast ASC to MayASC" true true "(R=1.000000,G=0.000000,B=0.009008,A=1.000000)"))))
    (:CastFailed
      (Development|PrintString "Cannot cast ASC to MayASC" true true "(R=1.000000,G=0.000000,B=0.009008,A=1.000000)"))))