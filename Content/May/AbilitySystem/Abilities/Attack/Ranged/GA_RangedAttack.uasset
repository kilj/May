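; Gameplay ability for a ranged attack that throws a flying stone projectile carrying a damage effect.
; On activation it picks a random attack from the avatar's character config, reached through the combat actor interface, and plays its montage.
; A gameplay event matching the attack's tag spawns the projectile from that attack's socket toward the facing target.
; The ability ends when the montage completes, is interrupted or is cancelled.
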(event Ability|EventActivateAbility
  (bind _ascombat_actor_interface (Utilities|Casting|CastToCombatActorInterface (Ability|GetAvatarActorfromActorInfo)))
  (bind _output_get (Variables|Internal|SetAvatarAsCombatActor _ascombat_actor_interface))
  (bind _output_get_2 (Variables|Default|SetAttackInfo (.OutItem (Utilities|Array|Random (Variables|/Script/May.CharacterConfig|GetAttacks (Class|CombatActorInterface|GetCharacterConfig _output_get))))))
  (|PlayMontageandWaitProxy "None" (.montage _output_get_2) 1.0 "None" true 1.0 0.0 false
    (:then
      (Ability|Tasks|WaitGameplayEvent (.tag (Variables|Default|GetAttackInfo)) 0
        (:EventReceived
          (Class|MayGameplayAbility|SpawnProjectileandAttachEffect "/Game/May/AbilitySystem/Abilities/Attack/Ranged/BP_FlyingStone.BP_FlyingStone_C" "/Game/May/AbilitySystem/Effects/GE_Damage.GE_Damage_C" (Variables|Default|GetDamage) (Class|CharacterConfig|GetAttackSocketLocation (Class|CombatActorInterface|GetCharacterConfig (Variables|Internal|GetAvatarAsCombatActor)) (.tag (Variables|Default|GetAttackInfo)) (.AsMay%20Character%20Base (Utilities|Casting|CastToMayCharacterBase (Variables|Internal|GetAvatarAsCombatActor)))) (Class|CombatActorInterface|GetFacingTarget (Variables|Internal|GetAvatarAsCombatActor))))))
    (:OnCompleted
      (Ability|EndAbility :!label _label))
    (:OnInterrupted
      (goto _label))
    (:OnCancelled
      (goto _label))))

(event Ability|EventOnEndAbility
  (params (bWasCancelled :type Boolean)))