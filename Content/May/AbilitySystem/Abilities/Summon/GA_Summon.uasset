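; GA_Summon is a gameplay ability that lets a combat character summon three random minions in front of itself.
; It picks a random summon entry from the avatar's character config, plays its montage and waits for that entry's gameplay event.
; The event spawns minions with default controllers and a Niagara ground effect at shuffled forward-cone locations.
; The ability ends after a fixed delay once the montage completes, is interrupted or is cancelled.
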(event Ability|EventActivateAbility
  (bind _ascombat_actor_interface (Utilities|Casting|CastToCombatActorInterface (Ability|GetAvatarActorfromActorInfo)))
  (bind _output_get (Variables|Default|SetAvatarAsCombatActor _ascombat_actor_interface))
  (bind _output_get_2 (Variables|Default|SetSummonInfo (.OutItem (Utilities|Array|Random (Variables|/Script/May.CharacterConfig|GetSummons (Class|CombatActorInterface|GetCharacterConfig _output_get))))))
  (|PlayMontageandWaitProxy "None" (.montage _output_get_2) 1.0 "None" true 1.0 0.0 false
    (:then
      (Ability|Tasks|WaitGameplayEvent (.tag (Variables|Default|GetSummonInfo)) 0
        (:EventReceived
          (bind _returnvalue (Class|MayGameplayAbility|GetSpawnLocationsinForwardConeEvenly 3 6e+01 1.2e+02 4e+02 false))
          (Utilities|Array|Shuffle _returnvalue)
          (for _array_element _returnvalue
            (Niagara|SpawnSystematLocation "/Game/May/Assets/Effects/Combat/NS_GroundSummon.NS_GroundSummon" _array_element "0, 0, 0" "1.000000,1.000000,1.000000" true true "AutoRelease")
            (bind _returnvalue_2 (Game|SpawnActorfromClass (.OutItem (Utilities|Array|Random (Variables|Default|GetMinionsToSpawn))) (Math|Transform|MakeTransform _array_element (Transformation|GetActorRotation (Ability|GetAvatarActorfromActorInfo))) "AlwaysSpawn" "MultiplyWithRoot" 0 0))
            (Pawn|SpawnDefaultController _returnvalue_2)))))
    (:OnCompleted
      (Utilities|FlowControl|Delay 5.0 :!label _label)
      (Ability|EndAbility))
    (:OnInterrupted
      (goto _label))
    (:OnCancelled
      (goto _label))))

(event Ability|EventOnEndAbility
  (params (bWasCancelled :type Boolean)))