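; GA_SpellBlink is a Gameplay Ability that teleports the avatar to the location under the player's click.
; TargetDataUnderClick supplies the hit location, then the Firebolt cast montage plays and its gameplay event triggers the teleport and a look-at rotation toward that location.
; The ability ends when the montage completes, is interrupted or is cancelled.
; Facing and projectile-spawn nodes are disconnected, and MaxDistance is unused, so the graph applies no range limit.
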(event Ability|EventActivateAbility
  (bind _datahandle (|TargetDataUnderClick)
    (:OnValidData
      (Variables|Default|SetTargetLocation (.Location (Collision|BreakHitResult (Ability|TargetData|GetHitResultfromTargetData _datahandle))))
      (Variables|Default|SetActor (Ability|GetAvatarActorfromActorInfo))
      (|PlayMontageandWaitProxy "None" "/Game/May/Assets/Characters/Aura/Animations/Abilities/AM_Cast_FireBolt.AM_Cast_FireBolt" 1.0 "None" true 1.0 0.0 false
        (:then
          (Ability|Tasks|WaitGameplayEvent "(TagName=\"Event.Montage.Firebolt\")" 0
            (:EventReceived
              (Transformation|SetActorLocation (Variables|Default|GetActor) (Variables|Default|GetTargetLocation) false true)
              (Transformation|SetActorRotation (Variables|Default|GetActor) (Math|Rotator|FindLookatRotation (.location (Transformation|GetActorTransform (Variables|Default|GetActor))) (Variables|Default|GetTargetLocation)) true))))
        (:OnCompleted
          (Ability|EndAbility :!label _label))
        (:OnInterrupted
          (goto _label))
        (:OnCancelled
          (goto _label))))))

(event Ability|EventOnEndAbility
  (params (bWasCancelled :type Boolean)))